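; BP_Fruit is a short-lived scoring fruit actor that appears as a banana, melon or apple.
; On BeginPlay, up to two separate rounded random rolls pick the variant by destroying the other two components, then the actor destroys itself after a delay.
; DestroyFruit adds its Score to the BP_ScoreBoard found in the level, spawns an explosion emitter at Core's location and removes the actor.
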(event Custom|DestroyFruit
  (bind _returnvalue (Actor|GetActorOfClass "/Game/BP_ScoreBoard.BP_ScoreBoard_C"))
  (Default|IncrementScore _returnvalue (Variables|Default|Getscore))
  (Effects|SpawnEmitteratLocation "/Game/Realistic_Starter_VFX_Pack_Vol2/Particles/Explosion/Explosion.Explosion" (Transformation|GetWorldLocation (Variables|Default|GetCore)) "0, 0, 0" "2.000000,2.000000,2.000000")
  (Actor|DestroyActor))

(event EventBeginPlay
  (bind _returnvalue (Math|Random|RandomFloatinRange 1.0 3.0))
  (bind _returnvalue_2 (Math|Float|Round _returnvalue))
  (if (== _returnvalue_2 1)
    ;[1 1 1] Banana
    (Components|DestroyComponent (Variables|Default|GetApple))
    (Components|DestroyComponent (Variables|Default|GetMelon))
    (elif (== _returnvalue_2 2)
      ;[1 1 1] Melon
      (Components|DestroyComponent (Variables|Default|GetApple))
      (Components|DestroyComponent (Variables|Default|GetBanana))
      (else
        ;[1 1 1] Banana
        (Components|DestroyComponent (Variables|Default|GetBanana))
        (Components|DestroyComponent (Variables|Default|GetMelon)))))
  (Utilities|FlowControl|Delay 1e+01)
  (Actor|DestroyActor))

(fn ConstructionScript)