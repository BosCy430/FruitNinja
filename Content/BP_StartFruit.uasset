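; BP_StartFruit is an apple actor that starts the game through the scoreboard.
; Its Start event finds BP_ScoreBoard, calls StartGame, then hides the fruit's component hierarchy and disables the apple mesh's collision.
; Reactivate shows the fruit again and restores query-only collision, so the same actor can be reused.
; Nothing in this Blueprint calls either event, so both are triggered from outside.
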(event Custom|Start
  (bind _returnvalue (Actor|GetActorOfClass "/Game/BP_ScoreBoard.BP_ScoreBoard_C"))
  (Default|StartGame _returnvalue)
  (Rendering|SetVisibility (Variables|Default|GetDefaultSceneRoot) false true)
  (Collision|SetCollisionEnabled (Variables|Default|Getapple_apple_whole) "NoCollision"))

(event Custom|Reactivate
  (Rendering|SetVisibility (Variables|Default|GetDefaultSceneRoot) true true)
  (Collision|SetCollisionEnabled (Variables|Default|Getapple_apple_whole) "QueryOnly"))

(fn ConstructionScript)