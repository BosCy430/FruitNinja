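; BP_FruitShooter is an actor that repeatedly launches apples from its position in the level.
; From BeginPlay it waits a random few seconds, spawns a BP_Apple at its Arrow component's location and rotation, and fires it with an impulse along the arrow's forward vector.
; The shot wires back into the random delay, so firing loops indefinitely without a timer.
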(event Custom|ShootFruits
  (bind _arrow (Variables|Default|GetArrow))
  (bind _returnvalue (Game|SpawnActorfromClass "/Game/BP_Apple.BP_Apple_C" (Math|Transform|MakeTransform (Transformation|GetWorldLocation _arrow) (Transformation|GetWorldRotation _arrow) "1.000000,1.000000,1.000000") "Undefined" "MultiplyWithRoot" 0 0))
  (Physics|AddImpulse (Variables|/Game/BP_Apple.BP_Apple_C|GetApple _returnvalue) (* (Math|Vector|GetForwardVector _arrow) 3.5e+03) "None" false)
  (Utilities|FlowControl|Delay (Math|Random|RandomFloatinRange 2.0 4.0))
  (CallFunction|ShootFruits))

(event EventBeginPlay
  (Utilities|FlowControl|Delay (Math|Random|RandomFloatinRange 2.0 4.0))
  (CallFunction|ShootFruits))

(fn ConstructionScript)