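; BP_Sword is a sword actor that slices fruit by overlap.
; Two box components, Box and Box1, run the same begin-overlap logic: a BP_Apple gets DestroyFruit, otherwise a BP_StartFruit gets Start.
; BeginPlay caches the level's BP_ScoreBoard via GetActorOfClass, though this graph never uses the reference.
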(event OnComponentBeginOverlap(Box1)
  (params (OverlappedComponent :type Primitive%20Component%20Object%20Reference) (OtherActor :type Actor%20Object%20Reference) (OtherComp :type Primitive%20Component%20Object%20Reference) (OtherBodyIndex :type Integer) (bFromSweep :type Boolean) (SweepResult :type Hit%20Result%20Structure%20%28by%20ref%29))
  (bind _asbp_apple (Utilities|Casting|CastToBP_Apple OtherActor)
    (:then
      (Default|DestroyFruit _asbp_apple))
    (:CastFailed
      (bind _asbp_start_fruit (Utilities|Casting|CastToBP_StartFruit OtherActor))
      (Default|Start _asbp_start_fruit))))

(event OnComponentBeginOverlap(Box)
  (params (OverlappedComponent :type Primitive%20Component%20Object%20Reference) (OtherActor :type Actor%20Object%20Reference) (OtherComp :type Primitive%20Component%20Object%20Reference) (OtherBodyIndex :type Integer) (bFromSweep :type Boolean) (SweepResult :type Hit%20Result%20Structure%20%28by%20ref%29))
  (bind _asbp_apple (Utilities|Casting|CastToBP_Apple OtherActor)
    (:then
      (Default|DestroyFruit _asbp_apple))
    (:CastFailed
      (bind _asbp_start_fruit (Utilities|Casting|CastToBP_StartFruit OtherActor))
      (Default|Start _asbp_start_fruit))))

(event EventBeginPlay
  (bind _returnvalue (Actor|GetActorOfClass "/Game/BP_ScoreBoard.BP_ScoreBoard_C"))
  (Variables|Default|SetscoreBoardRef _returnvalue))

(fn ConstructionScript)